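; BP_LevelEnd is the level goal trigger that tracks play time and collectibles, then ends the level when a living NewFleck_BP's capsule overlaps its box.
; A one-second Delay on Tick drives the minutes/seconds timer, and CollectibleGot increments the pickup count.
; On overlap, the game instance's IsStandard flag selects the standard or mini-golf end screen, which receives results and par targets, runs its star check and pauses the game.
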(event `CollectibleGot`
  (set `self.CollectiblesCollected` (+ (`self.CollectiblesCollected`) 1)))

(event `self.ReceiveTick`
  (params (DeltaSeconds :type "Float (single-precision)"))
  (`KismetSystemLibrary.Delay` 1.0)
  (bind _output_get (set `self.Seconds` (+ (`self.Seconds`) 1)))
  (if (> _output_get 59)
    (set `self.Minutes` (+ (`self.Minutes`) 1))
    (set `self.Seconds` 0)))

(event `self.Box.OnComponentBeginOverlap`
  (params (OverlappedComponent :type "PrimitiveComponent Object Reference") (OtherActor :type "Actor Object Reference") (OtherComp :type "PrimitiveComponent Object Reference") (OtherBodyIndex :type Integer) (bFromSweep :type Boolean) (SweepResult :type "HitResult Structure (by ref)"))
  (bind _returnvalue (`GameplayStatics.GetPlayerController` 0))
  (bind _asnew_fleck_bp (cast `/Game/AddedContent/MyBluePrints/NewFleck_BP` OtherActor))
  (if (== OtherComp (`Character.CapsuleComponent` _asnew_fleck_bp))
    (if (not (`/Game/AddedContent/MyBluePrints/NewFleck_BP.Dead` _asnew_fleck_bp))
      (bind _asnew_game_instance (cast `/Game/AddedContent/MyBluePrints/NewGameInstance` (`GameplayStatics.GetGameInstance`)))
      (if (`/Game/AddedContent/MyBluePrints/NewGameInstance.IsStandard` _asnew_game_instance)
        (bind _returnvalue_2 (`|CreateWidget` "/Game/UI/BPW_EndLevelScreen.BPW_EndLevelScreen_C"))
        (bind _output_get (set `self.EndLevelScreenRef` _returnvalue_2))
        (set `/Game/UI/BPW_EndLevelScreen.NewLevel` (`self.NextLevel`) _output_get)
        (set `/Game/UI/BPW_EndLevelScreen.Replay` (`self.CurrentLevel`) _output_get)
        (set `/Game/UI/BPW_EndLevelScreen.PlayerSeconds` (`self.Seconds`) _output_get)
        (set `/Game/UI/BPW_EndLevelScreen.PlayerMinutes` (`self.Minutes`) _output_get)
        (set `/Game/UI/BPW_EndLevelScreen.ParMinutes` (`self.LevelParMinutes`) _output_get)
        (set `/Game/UI/BPW_EndLevelScreen.ParSeconds` (`self.LevelParSeconds`) _output_get)
        (set `/Game/UI/BPW_EndLevelScreen.LevelNo` (`self.LevelNumber`) _output_get)
        (set `/Game/UI/BPW_EndLevelScreen.Collectible Counter` (`self.CollectiblesCollected`) _output_get)
        (`UserWidget.AddToViewport` _returnvalue_2 0)
        (`WidgetBlueprintLibrary.SetInputMode_UIOnlyEx` _returnvalue _returnvalue_2)
        (`/Game/UI/BPW_EndLevelScreen.StarCheck` _returnvalue_2)
        (`GameplayStatics.SetGamePaused` true)
        (else
          (bind _returnvalue_3 (`|CreateWidget` "/Game/UI/BPW_EndLevelScreenMiniGolf.BPW_EndLevelScreenMiniGolf_C"))
          (set `/Game/UI/BPW_EndLevelScreenMiniGolf.Level Star Shots` (`self.LevelParShots`) _returnvalue_3)
          (set `/Game/UI/BPW_EndLevelScreenMiniGolf.Total  Shots` (`self.ShotsCounted`) _returnvalue_3)
          (set `/Game/UI/BPW_EndLevelScreenMiniGolf.PlayerSeconds` (`self.Seconds`) _returnvalue_3)
          (set `/Game/UI/BPW_EndLevelScreenMiniGolf.PlayerMinutes` (`self.Minutes`) _returnvalue_3)
          (set `/Game/UI/BPW_EndLevelScreenMiniGolf.NewLevel` (`self.NextLevel`) _returnvalue_3)
          (set `/Game/UI/BPW_EndLevelScreenMiniGolf.Replay` (`self.CurrentLevel`) _returnvalue_3)
          (set `/Game/UI/BPW_EndLevelScreenMiniGolf.LevelNo` (`self.LevelNumber`) _returnvalue_3)
          (`UserWidget.AddToViewport` _returnvalue_3 0)
          (`WidgetBlueprintLibrary.SetInputMode_UIOnlyEx` _returnvalue null)
          (`/Game/UI/BPW_EndLevelScreenMiniGolf.MiniGolfStarCheck` _returnvalue_3)
          (`GameplayStatics.SetGamePaused` true)))
      (`Widget.RemoveFromParent` (`self.NewVar`)))))

(fn `UserConstructionScript`)