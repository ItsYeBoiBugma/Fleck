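; BP_THing is an unfinished placement Blueprint that adds static mesh instances in its Construction Script, with no active runtime logic.
; It loops over XCount, adding world-space instances at a 200-unit X offset from StartingPoint, seeded from the root transform.
; StartingPoint is reset to an empty value after each add, so the offset does not accumulate.
; Disconnected leftovers show attempts at nested-loop Y stepping, batch adding and spline-length spacing.
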(fn `UserConstructionScript`
  (locals (CurrentTransform :type "Transform Structure"))
  (bind _output_get (set `self.Starting Point` (`SceneComponent.K2_GetComponentToWorld` (`self.DefaultSceneRoot`))))
  (set `local.CurrentTransform` _output_get)
  (for _ (range (+ (`self.X Count`) 1))
    (`InstancedStaticMeshComponent.AddInstance` (`KismetMathLibrary.MakeTransform` (`KismetMathLibrary.MakeVector` (+ (.x (.location (`self.Starting Point`))) 200.0))) true)
    (set `self.Starting Point` (struct))))