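; BP_TrashBG builds a block of instanced static meshes, apparently background trash going by its name.
; Its construction script runs nested loops over YCount, XCount and ZCount, stepping at fixed spacing along negative X, Y and Z respectively from the root transform.
; Each step adds random roll and yaw picks from RandRotation to the running transform, varying instance orientation.
; The event graph has no live logic, and a spline-length calculation is left unused.
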(fn `UserConstructionScript`
  (locals (CurrentTransformX :type "Transform Structure") (CurrentTransformZ :type "Transform Structure"))
  (bind _currenttransformz (`local.CurrentTransformZ`))
  (bind _currenttransformx (`local.CurrentTransformX`))
  (bind _output (`|GetArrayItem` (`self.RandRotation`) (`KismetMathLibrary.RandomInteger` 3)))
  (bind _output_2 (`|GetArrayItem` (`self.RandRotation`) (`KismetMathLibrary.RandomInteger` 3)))
  (bind _output_3 (`|GetArrayItem` (`self.RandRotation`) (`KismetMathLibrary.RandomInteger` 3)))
  (bind _returnvalue (`KismetMathLibrary.MakeTransform` (+ (.location (`self.Starting Point`)) (-200.0 0.0 0.0)) (`KismetMathLibrary.MakeRotator` (+ (.roll (.rotation (`self.Starting Point`))) _output_2) (+ (.pitch (.rotation (`self.Starting Point`))) 0.0) (+ (.yaw (.rotation (`self.Starting Point`))) _output_2)) (.scale (`self.Starting Point`))))
  (bind _output_get (set `self.Starting Point` (`SceneComponent.K2_GetComponentToWorld` (`self.DefaultSceneRoot`))))
  (bind _output_get_2 (set `local.CurrentTransformZ` _output_get))
  (set `local.CurrentTransformX` _output_get_2)
  (for _ (range 1 (+ (`self.Y Count`) 1))
    (`InstancedStaticMeshComponent.AddInstance` (`self.InstancedStaticMesh`) _returnvalue true)
    (bind _output_get_3 (set `self.Starting Point` _returnvalue :!label _label))
    (for _ (range 1 (+ (`self.X Count`) 1))
      (`InstancedStaticMeshComponent.AddInstance` (`self.InstancedStaticMesh`) _currenttransformx true)
      (set `local.CurrentTransformX` (`KismetMathLibrary.MakeTransform` (+ (.location _currenttransformx) (0.0 -200.0 0.0)) (`KismetMathLibrary.MakeRotator` (+ (.roll (.rotation _currenttransformx)) _output_3) (+ (.pitch (.rotation _currenttransformx)) 0.0) (+ (.yaw (.rotation _currenttransformx)) _output_3)) (.scale _currenttransformx)))
      (for _ (range 1 (+ (`self.Z Count`) 1)) :!label _label_2
        (`InstancedStaticMeshComponent.AddInstance` (`self.InstancedStaticMesh`) _currenttransformz true)
        (set `local.CurrentTransformZ` (`KismetMathLibrary.MakeTransform` (+ (.location _currenttransformz) (0.0 0.0 -200.0)) (`KismetMathLibrary.MakeRotator` (+ (.roll (.rotation _currenttransformz)) _output) (+ (.pitch (.rotation _currenttransformz)) 0.0) (+ (.yaw (.rotation _currenttransformz)) _output)) (.scale _currenttransformz))))
      (set `local.CurrentTransformZ` (stale _output_get_4)))
    (bind _output_get_4 (set `local.CurrentTransformX` _output_get_3))
    (goto _label_2))
  (goto _label))