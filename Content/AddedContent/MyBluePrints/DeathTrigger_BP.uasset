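; DeathTrigger_BP is a trigger actor that kills Fleck, the NewFleck_BP actor, when it overlaps the trigger.
; On overlap it casts the other actor and calls its DeathAnimation, with no size check despite the graph comment.
; An unconnected chain holds an unused death sequence: destroy, sound, pause, kill widget with UI-only input, and HUD removal.
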(event `self.ReceiveActorBeginOverlap`
  (params (OtherActor :type "Actor Object Reference"))
  ;[1 1 1] Checks Fleck's size and kills him if too small
  (bind _asnew_fleck_bp (cast `/Game/AddedContent/MyBluePrints/NewFleck_BP` OtherActor))
  (`/Game/AddedContent/MyBluePrints/NewFleck_BP.Death Animation` _asnew_fleck_bp))

(fn `UserConstructionScript`)