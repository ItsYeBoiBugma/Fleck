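; NPC_BP is a patrolling hazard that kills the player's Fleck characters on contact.
; A timeline lerps it back and forth along Y from its start by TravelDistance, caching the current level name on each update.
; A capsule hit destroys Fleck_BP once, then shows the BPW_Kill widget with that level for replay and switches to UI-only input.
; Overlap with NewFleck_BP only destroys it; an OpenLevel call is left unwired.
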(event `self.ReceiveBeginPlay`
  (bind _output_get (set `self.Initial Location` (`self.K2_GetActorLocation`)))
  (set `self.Destination Location` (+ _output_get (`KismetMathLibrary.MakeVector` 0.0 (`self.TravelDistance`))))
  (bind (_direction _newtrack_0) (`Timeline|Timeline` :!label _label)
    (:`Update`
      (`self.K2_SetActorLocation` (`KismetMathLibrary.VLerp` (`self.Initial Location`) (`self.Destination Location`) _newtrack_0))
      (bind _returnvalue (`GameplayStatics.GetCurrentLevelName` true))
      (bind _output_get_2 (set `self.ActiveLevel` _returnvalue)))
    (:`Finished`
      (if (`self.Timeline Factor`)
        (set `self.Timeline Factor` false)
        (goto _label :!via `ReverseFromEnd`)
        (else
          (set `self.Timeline Factor` true)
          (goto _label :!via `PlayFromStart`))))))

(event `self.CapsuleComponent.OnComponentHit`
  (params (HitComponent :type "PrimitiveComponent Object Reference") (OtherActor :type "Actor Object Reference") (OtherComp :type "PrimitiveComponent Object Reference") (NormalImpulse :type "Vector Structure") (Hit :type "HitResult Structure (by ref)"))
  (bind _asfleck_bp (cast `/Game/AddedContent/MyBluePrints/Fleck_BP` OtherActor))
  (`/Engine/EditorBlueprintResources/StandardMacros.DoOnce` false
    (:`Completed`
      (`self.K2_DestroyActor` _asfleck_bp)
      (bind _returnvalue (`|CreateWidget` "/Game/UI/BPW_Kill.BPW_Kill_C"))
      (`UserWidget.AddToViewport` _returnvalue 0)
      (set `/Game/UI/BPW_Kill.ReplayName` (`KismetStringLibrary.Conv_StringToName` (stale `self.ReceiveBeginPlay` _output_get_2)) _returnvalue)
      (`WidgetBlueprintLibrary.SetInputMode_UIOnlyEx` (`GameplayStatics.GetPlayerController` 0) null))))

(event `self.ReceiveActorBeginOverlap`
  (params (OtherActor :type "Actor Object Reference"))
  ;[1 1 1] Kills Fleck
  (bind _asnew_fleck_bp (cast `/Game/AddedContent/MyBluePrints/NewFleck_BP` OtherActor))
  (`self.K2_DestroyActor` _asnew_fleck_bp))

(fn `UserConstructionScript`)