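; Fleck player Blueprint that the player launches by touch-dragging and releasing, with a launch meter widget added at BeginPlay.
; While dragging, Tick turns the mouse offset from the press point into clamped Y/Z impulses and spawns PredictionPath_BP actors along a predicted arc, which uses the unclamped values.
; A downward line trace sets IsGrounded; release stops aiming and applies the impulse to the capsule only when grounded.
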(event `self.ReceiveTick`
  (params (DeltaSeconds :type "Float (single-precision)"))
  (bind _returnvalue (`SceneComponent.K2_GetComponentLocation` (`self.Mesh`)))
  ;[1 1 1] Ground Check
  (bind (_outhit _returnvalue_2) (`KismetSystemLibrary.LineTraceSingleForObjects` :`Start` _returnvalue :`End` (+ _returnvalue (* (`KismetMathLibrary.Vector_Down`) (`self.Ground Check Distance`))) :`ObjectTypes` (`self.Object Types`) :`DrawDebugType` "ForOneFrame" :`DrawTime` 1.0))
  (if _returnvalue_2
    (set `self.IsGrounded` true)
    (else
      (set `self.IsGrounded` false)))
  (if (`self.ShouldTrace`)
    (bind _returnvalue_3 (`WidgetLayoutLibrary.GetMousePositionOnViewport`))
    (`SceneComponent.K2_SetWorldLocation` (`self.Launch Point`) (`GameplayStatics.DeprojectScreenToWorld` null _returnvalue_3) false false)
    (bind (_returnvalue_x _returnvalue_y) (`KismetMathLibrary.BreakVector2D` (- _returnvalue_3 (`self.Initial Click Position`))))
    (bind _returnvalue_4 (* _returnvalue_x (`self.Y Velocity Multiplier`)))
    (set `self.Clamped Y Impulse` (`KismetMathLibrary.FClamp` _returnvalue_4 -1200.0 1200.0))
    (bind _returnvalue_5 (* _returnvalue_y (`self.X Velocity Multiplier`)))
    (set `self.Clamped Z Impulse` (`KismetMathLibrary.FClamp` _returnvalue_5 -1200.0 1200.0))
    (bind (_outhit_2 _outpathpositions) (`GameplayStatics.Blueprint_PredictProjectilePath_ByTraceChannel` :`StartPos` (`SceneComponent.K2_GetComponentLocation` (`self.Prediction Path`)) :`LaunchVelocity` (`KismetMathLibrary.MakeVector` 0.0 _returnvalue_4 _returnvalue_5) :`ProjectileRadius` 2.0 :`DrawDebugTime` 1.0 :`SimFrequency` 10.0 :`MaxSimTime` 1.0 :`OverrideGravityZ` (`self.Override Gravity Z`))) ; Changed Override Gravity from 50 to 0
    (for _array_element _outpathpositions
      (`|SpawnActorFromClass` "/Game/Blueprints/PlayerController/PredictionPath_BP.PredictionPath_BP_C" (`KismetMathLibrary.MakeTransform` _array_element) "Undefined" "MultiplyWithRoot" null null))))

(event `InputTouch`
  (params (Location :type "Vector Structure") (FingerIndex :type "ETouchIndex Enum"))
  (:`Pressed`
    (set `self.ShouldTrace` true)
    (bind _returnvalue (`WidgetLayoutLibrary.GetMousePositionOnViewport`))
    (set `self.Initial Click Position` _returnvalue))
  (:`Released`
    (if (`self.IsGrounded`)
      (set `self.ShouldTrace` false)
      (`PrimitiveComponent.AddImpulse` (`self.CapsuleComponent`) (`KismetMathLibrary.MakeVector` 0.0 (`self.Clamped Y Impulse`) (`self.Clamped Z Impulse`)) "None" true))))

(event `self.ReceiveBeginPlay`
  (bind _returnvalue (`|CreateWidget` "/Game/AddedContent/MyBluePrints/FleckLaunchMeter_BP.FleckLaunchMeter_BP_C"))
  (`UserWidget.AddToViewport` _returnvalue 0))

(fn `UserConstructionScript`)