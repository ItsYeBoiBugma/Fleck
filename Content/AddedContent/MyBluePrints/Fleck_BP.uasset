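; Fleck_BP is a touch-drag launcher that flings its BasicSphere with a predicted trajectory preview.
; Touch press records the start position; the drag offset sets velocity, with scaled screen X driving world Y and screen Y driving Z.
; While held, Tick prints the X value, predicts the path from LaunchPoint and spawns PredictionPath_BP markers along it.
; Release stops tracing and applies the offset as a velocity-change impulse.
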(event `self.ReceiveTick`
  (params (DeltaSeconds :type "Float (single-precision)"))
  (if (`self.ShouldTrace`)
    (bind _returnvalue (`WidgetLayoutLibrary.GetMousePositionOnViewport`))
    (bind (_returnvalue_x _returnvalue_y) (`KismetMathLibrary.BreakVector2D` (- _returnvalue (`self.InitialClickPosition`))))
    (bind _returnvalue_2 (* _returnvalue_x (`self.VelocityMultiplier`)))
    ;[1 1 1] Printing Difference in X Value * Velocity Multiplier
    (`KismetSystemLibrary.PrintString` (`KismetStringLibrary.Concat_StrStr` "X :" (`KismetStringLibrary.Conv_DoubleToString` _returnvalue_2)))
    (bind (_outhit _outpathpositions) (`GameplayStatics.Blueprint_PredictProjectilePath_ByTraceChannel` :`StartPos` (`SceneComponent.K2_GetComponentLocation` (`self.Launch Point`)) :`LaunchVelocity` (`KismetMathLibrary.MakeVector` 0.0 _returnvalue_2 _returnvalue_y) :`ProjectileRadius` 2.0 :`DrawDebugTime` 1.0 :`SimFrequency` 10.0 :`MaxSimTime` 1.0 :`OverrideGravityZ` 50.0))
    (for _array_element _outpathpositions
      (`|SpawnActorFromClass` "/Game/ThirdPerson/Blueprints/PredictionPath_BP.PredictionPath_BP_C" (`KismetMathLibrary.MakeTransform` _array_element) "Undefined" "MultiplyWithRoot" null null))))

(event `InputTouch`
  (params (Location :type "Vector Structure") (FingerIndex :type "ETouchIndex Enum"))
  (:`Pressed`
    (set `self.ShouldTrace` true)
    (bind _returnvalue (`WidgetLayoutLibrary.GetMousePositionOnViewport`))
    (set `self.InitialClickPosition` _returnvalue))
  (:`Released`
    (set `self.ShouldTrace` false)
    (bind (_returnvalue_x _returnvalue_y) (`KismetMathLibrary.BreakVector2D` (- (stale `self.ReceiveTick` _returnvalue) (`self.InitialClickPosition`))))
    (`PrimitiveComponent.AddImpulse` (`self.BasicSphere`) (`KismetMathLibrary.MakeVector` 0.0 (* _returnvalue_x (`self.VelocityMultiplier`)) _returnvalue_y) "None" true)))

(fn `UserConstructionScript`)